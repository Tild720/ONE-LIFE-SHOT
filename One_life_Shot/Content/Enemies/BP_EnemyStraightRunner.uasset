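; Straight-running enemy that locks a flat direction toward the player's position at BeginPlay and runs along it without re-aiming.
; Blocking hits against BP_ThirdPersonCharacter call FailRun, while overlaps or hits with GameTraceChannel1 objects kill the enemy.
; Death disables movement and collision, spawns a BP_PistolPickup that returns to the player, and sets lifespan to cover the death animation.
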(event `self.ReceiveBeginPlay`
  (bind _returnvalue (`GameplayStatics.GetPlayerPawn` 0))
  (bind _weaponmesh (`self.WeaponMesh`))
  (`PrimitiveComponent.SetCollisionEnabled` _weaponmesh "NoCollision")
  (`SceneComponent.K2_AttachToComponent` _weaponmesh (`self.Mesh`) "WeaponSocket_R" "SnapToTarget" "SnapToTarget" "KeepRelative" false)
  (`PrimitiveComponent.SetCollisionResponseToChannel` (`self.CapsuleComponent`) "ECC_GameTraceChannel1" "ECR_Overlap")
  (`/Engine/EditorBlueprintResources/StandardMacros.IsValid` _returnvalue
    (:`Is Valid`
      (set `self.TravelDirection` (`KismetMathLibrary.Vector_Normal2D` (- (`self.K2_GetActorLocation` _returnvalue) (`self.K2_GetActorLocation`))))
      (`self.K2_SetActorRotation` (`KismetMathLibrary.MakeRotFromX` (`self.TravelDirection`)))
      (`SkeletalMeshComponent.PlayAnimation` (`self.Mesh`) (`self.RunAnimation`) true))
    (:`Is Not Valid`
      (`self.SetActorTickEnabled` false))))

(event `self.ReceiveTick`
  (params (DeltaSeconds :type "Float (single-precision)"))
  (if (not (`self.Dead`))
    (set `CharacterMovementComponent.MaxWalkSpeed` (select `bool` (> (`self.MoveSpeed`) 0.0) :`false` 0.0 :`true` (`self.MoveSpeed`)) (`self.CharacterMovement`))
    (`self.AddMovementInput` (`self.TravelDirection`) 1.0 true)))

(event `self.ReceiveActorBeginOverlap`
  (params (OtherActor :type "Actor Object Reference"))
  (for _array_element (`self.GetOverlappingComponents`)
    (if (`|EnumEquality` (`PrimitiveComponent.GetCollisionObjectType` _array_element) (enumliteral `ECollisionChannel` "ECC_GameTraceChannel1"))
      (`self.Die`))))

(event `self.ReceiveHit`
  (params (MyComp :type "PrimitiveComponent Object Reference") (Other :type "Actor Object Reference") (OtherComp :type "PrimitiveComponent Object Reference") (bSelfMoved :type Boolean) (HitLocation :type "Vector Structure") (HitNormal :type "Vector Structure") (NormalImpulse :type "Vector Structure") (Hit :type "HitResult Structure (by ref)"))
  (if (`|EnumEquality` (`PrimitiveComponent.GetCollisionObjectType` OtherComp) (enumliteral `ECollisionChannel` "ECC_GameTraceChannel1"))
    (`self.Die`)
    (else
      (bind _asbp_third_person_character (cast `/Game/ThirdPerson/Blueprints/BP_ThirdPersonCharacter` Other))
      (`/Game/ThirdPerson/Blueprints/BP_ThirdPersonCharacter.FailRun` _asbp_third_person_character))))

(fn `Die`
  (bind _deathanimation (`self.DeathAnimation`))
  (if (not (`self.Dead`))
    (set `self.Dead` true)
    (`CharacterMovementComponent.DisableMovement` (`self.CharacterMovement`))
    (`self.SetActorTickEnabled` false)
    (`self.SetActorEnableCollision` false)
    (bind _returnvalue (`|SpawnActorFromClass` "/Game/Weapons/Pistol/BP_PistolPickup.BP_PistolPickup_C" (`self.GetTransform`) "AlwaysSpawn" "MultiplyWithRoot" null null))
    (if (`KismetSystemLibrary.IsValid` _returnvalue)
      (`/Game/Weapons/Pistol/BP_PistolPickup.ReturnToPlayer` _returnvalue))
    (`/Engine/EditorBlueprintResources/StandardMacros.IsValid` _deathanimation
      (:`Is Valid`
        (`SkeletalMeshComponent.PlayAnimation` (`self.Mesh`) _deathanimation false)
        (`self.SetLifeSpan` (+ (`AnimationAsset.GetPlayLength` _deathanimation) 0.1)))
      (:`Is Not Valid`
        (`self.SetLifeSpan` 0.1)))))

(fn `UserConstructionScript`)
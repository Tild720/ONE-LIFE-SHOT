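; Enemy spawn point for a runner level that periodically spawns random enemies from pools and intervals chosen by the ProgressManager's current stage.
; A looping timer checks the player's distance along the start-to-end track axis, spawning only within an activation window and retiring permanently once the player gets too close or passes.
; Spawning skips one stage, caps living enemies, sets their lifespan and can override straight-runner move speed.
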(event `self.ReceiveBeginPlay`
  (set `self.NextSpawnTime` (+ (`KismetSystemLibrary.GetGameTimeInSeconds`) (select `bool` (> (`self.SpawnDelay`) 0.0) :`false` 0.0 :`true` (`self.SpawnDelay`))))
  (`KismetSystemLibrary.K2_SetTimer` self "SpawnNext" 0.2 true))

(fn `RefreshStageSettings`
  (set `self.ActivePool` (select `bool` (`|EnumEquality` (`/Game/Runner/BP_RunnerProgress.CurrentStage` (`self.ProgressManager`)) (enumliteral `/Game/Runner/E_RunnerStage` "NewEnumerator3")) :`false` (select `bool` (`|EnumEquality` (`/Game/Runner/BP_RunnerProgress.CurrentStage` (`self.ProgressManager`)) (enumliteral `/Game/Runner/E_RunnerStage` "NewEnumerator2")) :`false` (select `bool` (`|EnumEquality` (`/Game/Runner/BP_RunnerProgress.CurrentStage` (`self.ProgressManager`)) (enumliteral `/Game/Runner/E_RunnerStage` "NewEnumerator1")) :`false` (`self.EarlyEnemyPool`) :`true` (`self.MiddleEnemyPool`)) :`true` (`self.LateEnemyPool`)) :`true` (`self.FinalEnemyPool`)))
  (set `self.ActiveInterval` (select `bool` (`|EnumEquality` (`/Game/Runner/BP_RunnerProgress.CurrentStage` (`self.ProgressManager`)) (enumliteral `/Game/Runner/E_RunnerStage` "NewEnumerator3")) :`false` (select `bool` (`|EnumEquality` (`/Game/Runner/BP_RunnerProgress.CurrentStage` (`self.ProgressManager`)) (enumliteral `/Game/Runner/E_RunnerStage` "NewEnumerator2")) :`false` (select `bool` (`|EnumEquality` (`/Game/Runner/BP_RunnerProgress.CurrentStage` (`self.ProgressManager`)) (enumliteral `/Game/Runner/E_RunnerStage` "NewEnumerator1")) :`false` (`self.EarlyInterval`) :`true` (`self.MiddleInterval`)) :`true` (`self.LateInterval`)) :`true` (`self.FinalInterval`))))

(fn `SpawnNext`
  (if (`self.Enabled`)
    (`/Engine/EditorBlueprintResources/StandardMacros.IsValid` (`self.ProgressManager`)
      (:`Is Valid`
        (`self.UpdateSpawnWindow`)
        (if (`self.SpawnWindowOpen`)
          (if (not (`|EnumEquality` (`/Game/Runner/BP_RunnerProgress.CurrentStage` (`self.ProgressManager`)) (enumliteral `/Game/Runner/E_RunnerStage` "NewEnumerator4")))
            (`self.RefreshStageSettings`)
            (set `self.NextSpawnTime` (select `bool` (< (`self.NextSpawnTime`) (+ (`KismetSystemLibrary.GetGameTimeInSeconds`) (`KismetMathLibrary.FClamp` (`self.ActiveInterval`) 0.1 3600.0))) :`false` (+ (`KismetSystemLibrary.GetGameTimeInSeconds`) (`KismetMathLibrary.FClamp` (`self.ActiveInterval`) 0.1 3600.0)) :`true` (`self.NextSpawnTime`)))
            (if (>= (`KismetSystemLibrary.GetGameTimeInSeconds`) (`self.NextSpawnTime`))
              (set `self.NextSpawnTime` (+ (`KismetSystemLibrary.GetGameTimeInSeconds`) (`KismetMathLibrary.FClamp` (`self.ActiveInterval`) 0.1 3600.0)))
              (`KismetArrayLibrary.Array_Clear` (`self.Survivors`))
              (for _array_element (`self.AliveEnemies`)
                (`/Engine/EditorBlueprintResources/StandardMacros.IsValid` _array_element
                  (:`Is Valid`
                    (`KismetArrayLibrary.Array_Add` (`self.Survivors`) _array_element))))
              (set `self.AliveEnemies` (`self.Survivors`))
              (set `self.AliveCount` (`KismetArrayLibrary.Array_Length` (`self.AliveEnemies`)))
              (if (and (< (`self.AliveCount`) (`self.MaxAliveEnemies`)) (> (`KismetArrayLibrary.Array_Length` (`self.ActivePool`)) 0))
                (set `self.SelectedEnemyClass` (`KismetArrayLibrary.Array_Random` (`self.ActivePool`)))
                (if (`KismetSystemLibrary.IsValidClass` (`self.SelectedEnemyClass`))
                  (bind _returnvalue (`|SpawnActorFromClass` (`self.SelectedEnemyClass`) (`self.GetTransform`) "AdjustIfPossibleButDontSpawnIfColliding" "MultiplyWithRoot" self null))
                  (`/Engine/EditorBlueprintResources/StandardMacros.IsValid` _returnvalue
                    (:`Is Valid`
                      (`KismetArrayLibrary.Array_Add` (`self.AliveEnemies`) _returnvalue)
                      (`self.SetLifeSpan` _returnvalue (`self.EnemyLifetime`))
                      (if (`self.UseSpawnSpeedOverride`)
                        (bind _asbp_enemy_straight_runner (cast `/Game/Enemies/BP_EnemyStraightRunner` _returnvalue))
                        (set `/Game/Enemies/BP_EnemyStraightRunner.MoveSpeed` (`KismetMathLibrary.FClamp` (`self.SpawnSpeed`) 100.0 2000.0) _asbp_enemy_straight_runner)))))))))))))

(fn `UpdateSpawnWindow`
  (bind _returnvalue (`KismetMathLibrary.Dot_VectorVector` (- (`self.K2_GetActorLocation`) (`self.K2_GetActorLocation` (`GameplayStatics.GetPlayerPawn` 0))) (`KismetMathLibrary.Vector_Normal2D` (- (`self.K2_GetActorLocation` (`/Game/Runner/BP_RunnerProgress.EndPoint` (`self.ProgressManager`))) (`self.K2_GetActorLocation` (`/Game/Runner/BP_RunnerProgress.StartPoint` (`self.ProgressManager`)))))))
  (set `self.SpawnWindowOpen` false)
  (if (not (`self.SpawnRetired`))
    (if (<= _returnvalue (`self.SpawnMinimumAhead`))
      (set `self.SpawnRetired` true)
      (`KismetSystemLibrary.K2_ClearTimer` self "SpawnNext")
      (elif (<= _returnvalue (`self.SpawnActivationDistance`))
        (set `self.SpawnWindowOpen` true)))))

(fn `UserConstructionScript`)
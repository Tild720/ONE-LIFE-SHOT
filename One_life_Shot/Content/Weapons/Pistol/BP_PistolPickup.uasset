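; Weapon pickup that shows a pistol, rifle, sniper or cylinder mesh by WeaponKind and equips that weapon on the player.
; A looping timer polls player distance against PickupRadius rather than using overlaps, then calls EquipPistol on a living character and destroys itself on success.
; ReturnToPlayer starts a timed lerp homing the pickup to just below the player's location, then retries acquisition on arrival.
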(event `self.ReceiveBeginPlay`
  (`self.ConfigurePickup`)
  (`KismetSystemLibrary.K2_SetTimer` self "TryAcquire" 0.08 true true))

(event `self.PickupRange.OnComponentBeginOverlap`
  (params (OverlappedComponent :type "PrimitiveComponent Object Reference") (OtherActor :type "Actor Object Reference") (OtherComp :type "PrimitiveComponent Object Reference") (OtherBodyIndex :type Integer) (bFromSweep :type Boolean) (SweepResult :type "HitResult Structure (by ref)"))
  (cast `/Game/ThirdPerson/Blueprints/BP_ThirdPersonCharacter` OtherActor))

(fn `ConfigurePickup`
  (bind _weaponkind (`self.WeaponKind`))
  (bind _pickupmesh (`self.PickupMesh`))
  (if (== _weaponkind 0)
    (`StaticMeshComponent.SetStaticMesh` _pickupmesh "/Game/Characters/KayKit/Assets/fbx/Gun_Pistol.Gun_Pistol")
    (`SceneComponent.SetRelativeScale3D` _pickupmesh (0.75 0.75 0.75))
    (`SceneComponent.K2_SetRelativeRotation` :`self` _pickupmesh :`bTeleport` true)
    (elif (== _weaponkind 1)
      (`StaticMeshComponent.SetStaticMesh` _pickupmesh "/Game/Characters/KayKit/Assets/fbx/Gun_Rifle.Gun_Rifle")
      (`SceneComponent.SetRelativeScale3D` _pickupmesh (0.9 0.48 0.85))
      (`SceneComponent.K2_SetRelativeRotation` :`self` _pickupmesh :`bTeleport` true)
      (elif (== _weaponkind 2)
        (`StaticMeshComponent.SetStaticMesh` _pickupmesh "/Game/Characters/KayKit/Assets/fbx/Gun_Sniper.Gun_Sniper")
        (`SceneComponent.SetRelativeScale3D` _pickupmesh (0.75 0.75 0.75))
        (`SceneComponent.K2_SetRelativeRotation` :`self` _pickupmesh :`bTeleport` true)
        (elif (== _weaponkind 3)
          (`StaticMeshComponent.SetStaticMesh` _pickupmesh "/Engine/BasicShapes/Cylinder.Cylinder")
          (`SceneComponent.SetRelativeScale3D` _pickupmesh (0.22 0.22 0.9))
          (`SceneComponent.K2_SetRelativeRotation` _pickupmesh (struct :`Roll` 90) false true))))))

(fn `ReturnToPlayer`
  (set `self.Returning` true)
  (set `self.ReturnStart` (`self.K2_GetActorLocation`))
  (set `self.ReturnStartTime` (`KismetSystemLibrary.GetGameTimeInSeconds`))
  (`KismetSystemLibrary.K2_SetTimer` self "UpdateReturn" 0.02 true true))

(fn `TryAcquire`
  (bind _returnvalue (`GameplayStatics.GetPlayerPawn` 0))
  (if (not (`self.Consumed`))
    (if (not (`self.Returning`))
      (if (`KismetSystemLibrary.IsValid` _returnvalue)
        (if (<= (`self.GetDistanceTo` _returnvalue) (`self.PickupRadius`))
          (bind _asbp_third_person_character (cast `/Game/ThirdPerson/Blueprints/BP_ThirdPersonCharacter` _returnvalue))
          (if (not (`/Game/ThirdPerson/Blueprints/BP_ThirdPersonCharacter.Dead` _asbp_third_person_character))
            (set `/Game/ThirdPerson/Blueprints/BP_ThirdPersonCharacter.NextWeaponKind` (`self.WeaponKind`) _asbp_third_person_character)
            (bind _success (`/Game/ThirdPerson/Blueprints/BP_ThirdPersonCharacter.EquipPistol` _asbp_third_person_character))
            (if _success
              (set `self.Consumed` true)
              (`GameplayStatics.PlaySound2D` "/Game/Weapons/Pistol/Audio/SW_WeaponPickup.SW_WeaponPickup" 1.0 1.0 0.0 null null false)
              (`self.K2_DestroyActor`))))))))

(fn `UpdateReturn`
  (bind _returnvalue (`GameplayStatics.GetPlayerPawn` 0))
  (bind _returnvalue_2 (`KismetMathLibrary.FClamp` (/ (- (`KismetSystemLibrary.GetGameTimeInSeconds`) (`self.ReturnStartTime`)) (`KismetMathLibrary.FClamp` (`self.ReturnDuration`) 0.1 2.0))))
  (if (`KismetSystemLibrary.IsValid` _returnvalue)
    (`self.K2_SetActorLocation` (`KismetMathLibrary.VLerp` (`self.ReturnStart`) (- (`self.K2_GetActorLocation` _returnvalue) (`KismetMathLibrary.MakeVector` 0.0 0.0 55.0)) _returnvalue_2) false true)
    (if (>= _returnvalue_2 1.0)
      (`KismetSystemLibrary.K2_ClearTimer` self "UpdateReturn")
      (set `self.Returning` false)
      (`self.TryAcquire`))
    (else
      (`KismetSystemLibrary.K2_ClearTimer` self "UpdateReturn")
      (set `self.Returning` false))))

(fn `UserConstructionScript`
  (`self.ConfigurePickup`)
  (`SphereComponent.SetSphereRadius` (`self.PickupRange`) (`self.PickupRadius`) true))
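; Single-shot pistol that fires a projectile toward the mouse cursor, with an optional unlimited-ammo mode.
; Fire aims at the cursor's trace hit on steep surfaces, otherwise where the cursor ray crosses a horizontal plane at muzzle height, keeping shots level.
; A successful shot updates ammo, ejects a casing, and triggers a timed muzzle light, camera shake, sound and particles.
; It then sets the ammo HUD to empty, even with unlimited ammo.
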(fn `ClearMuzzleLight`
  (`LightComponent.SetIntensity` (`self.MuzzleLight`) 0.0))

(fn `Fire`
  (bind _returnvalue (`GameplayStatics.GetPlayerController` 0))
  (bind _returnvalue_2 (`self.GetInstigator`))
  (bind _unlimitedammo (`self.UnlimitedAmmo`))
  (bind _weaponmesh (`self.WeaponMesh`))
  (bind (_worldlocation _worlddirection _returnvalue_3) (`PlayerController.DeprojectMousePositionToWorld` _returnvalue))
  (bind _returnvalue_4 (`SceneComponent.GetSocketLocation` (`self.WeaponMesh`) "Muzzle"))
  (bind _returnvalue_5 (+ _worldlocation (* _worlddirection (`KismetMathLibrary.MakeVector` 100000.0 100000.0 100000.0))))
  (if (or (> (`self.Ammo`) 0) _unlimitedammo)
    (if _returnvalue_3
      (bind (_outhit _returnvalue_6) (`KismetSystemLibrary.LineTraceSingle` _worldlocation _returnvalue_5 "TraceTypeQuery1" false (`|MakeArray` _returnvalue_2 :!type "Actor Object Reference")))
      (bind (_bblockinghit _binitialoverlap _time _distance _location _impactpoint _normal _impactnormal) (`GameplayStatics.BreakHitResult` _outhit))
      (bind _returnvalue_7 (`|SpawnActorFromClass` "/Game/Weapons/Pistol/BP_BulletProjectile.BP_BulletProjectile_C" (`KismetMathLibrary.MakeTransform` _returnvalue_4 (`KismetMathLibrary.FindLookAtRotation` _returnvalue_4 (`KismetMathLibrary.SelectVector` _impactpoint (`.Intersection` (`KismetMathLibrary.LinePlaneIntersection_OriginNormal` _worldlocation _returnvalue_5 _returnvalue_4 (`KismetMathLibrary.MakeVector` 0.0 0.0 1.0))) (and _returnvalue_6 (< (`KismetMathLibrary.Abs` (.z _impactnormal)) 0.7)))) (`KismetMathLibrary.MakeVector` 1.0 1.0 1.0)) "AlwaysSpawn" "MultiplyWithRoot" self _returnvalue_2))
      (if (`KismetSystemLibrary.IsValid` _returnvalue_7)
        (set `self.Ammo` (`KismetMathLibrary.SelectInt` 1 0 _unlimitedammo))
        (`self.FlashMuzzleLight`)
        (`|SpawnActorFromClass` "/Game/Weapons/Pistol/BP_PistolCasing.BP_PistolCasing_C" (`KismetMathLibrary.MakeTransform` (`KismetMathLibrary.TransformLocation` (`SceneComponent.K2_GetComponentToWorld` _weaponmesh) (`KismetMathLibrary.MakeVector` 10.0 25.0 15.0)) (`SceneComponent.K2_GetComponentRotation` _weaponmesh) (`KismetMathLibrary.MakeVector` 1.0 1.0 1.0)) "AlwaysSpawn" "MultiplyWithRoot" null null)
        (`PlayerController.ClientStartCameraShake` :`self` _returnvalue :`Shake` "/Game/Weapons/Pistol/CS_PistolFire.CS_PistolFire_C" :`Scale` (`self.FireShakeScale`))
        (`GameplayStatics.PlaySoundAtLocation` (`self.FireSound`) _returnvalue_4 (struct) 1.0 1.0 0.0 null null null null)
        (`GameplayStatics.SpawnEmitterAtLocation` (`self.MuzzleEffect`) _returnvalue_4 (struct) (`KismetMathLibrary.MakeVector` 1.0 1.0 1.0))
        (bind _asbp_ammo_hud (cast `/Game/ThirdPerson/Blueprints/BP_AmmoHUD` (`PlayerController.GetHUD` (`GameplayStatics.GetPlayerController` 0))))
        (set `/Game/ThirdPerson/Blueprints/BP_AmmoHUD.AmmoLabel` "0/1" _asbp_ammo_hud)
        (set `/Game/ThirdPerson/Blueprints/BP_AmmoHUD.StatusLabel` "EMPTY - DODGE / GET A WEAPON" _asbp_ammo_hud)))))

(fn `FlashMuzzleLight`
  (`LightComponent.SetIntensity` (`self.MuzzleLight`) (`self.MuzzleLightIntensity`))
  (`KismetSystemLibrary.K2_SetTimer` self "ClearMuzzleLight" (`self.MuzzleLightDuration`)))

(fn `UserConstructionScript`)
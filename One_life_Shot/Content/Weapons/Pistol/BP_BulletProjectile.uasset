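; Shared player projectile for pistol, shotgun, sniper and rocket shots, with a tracer that stretches to a capped length.
; ConfigureProjectile sets speed and range-based lifetime per WeaponKind; sniper rounds disable collision.
; Bullets flag tagged targets or kill runner enemies, with impact effects.
; Rockets detonate on contact or range timeout, dealing radial damage and building a timer-animated core, floor ring and camera-facing flare from runtime-added meshes.
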(event `self.ReceiveBeginPlay`
  (bind _projectilemovement (`self.ProjectileMovement`))
  (bind _projectilespeed (`self.ProjectileSpeed`))
  (bind _collision (`self.Collision`))
  (set `self.TrailStartLocation` (`self.K2_GetActorLocation`))
  (set `ProjectileMovementComponent.MaxSpeed` _projectilespeed _projectilemovement)
  (`ProjectileMovementComponent.SetVelocityInLocalSpace` _projectilemovement (`KismetMathLibrary.MakeVector` _projectilespeed))
  (`PrimitiveComponent.IgnoreActorWhenMoving` _collision (`self.GetInstigator`) true)
  (`PrimitiveComponent.IgnoreActorWhenMoving` _collision (`self.GetOwner`) true))

(event `self.ReceiveTick`
  (params (DeltaSeconds :type "Float (single-precision)"))
  (bind _maxtraillength (`self.MaxTrailLength`))
  (bind _tracer (`self.Tracer`))
  (bind _returnvalue (`KismetMathLibrary.Vector_Distance` (`self.K2_GetActorLocation`) (`self.TrailStartLocation`)))
  (bind _returnvalue_2 (`KismetMathLibrary.FClamp` _returnvalue 0.0 _maxtraillength))
  (`SceneComponent.SetRelativeScale3D` _tracer (`KismetMathLibrary.MakeVector` 0.035 0.035 (/ _returnvalue_2 100.0)))
  (`SceneComponent.K2_SetRelativeLocation` _tracer (`KismetMathLibrary.MakeVector` (* _returnvalue_2 -0.5)) false false)
  (if (>= _returnvalue _maxtraillength)
    (`self.SetActorTickEnabled` false)))

(event `self.Collision.OnComponentHit`
  (params (HitComponent :type "PrimitiveComponent Object Reference") (OtherActor :type "Actor Object Reference") (OtherComp :type "PrimitiveComponent Object Reference") (NormalImpulse :type "Vector Structure") (Hit :type "HitResult Structure (by ref)"))
  (bind _returnvalue (`self.K2_GetActorLocation`))
  (bind (_bblockinghit _binitialoverlap _time _distance _location _impactpoint _normal _impactnormal) (`GameplayStatics.BreakHitResult` Hit))
  (`self.HandleWeaponHit`)
  (if (== (`self.WeaponKind`) 3)
    (`self.Detonate`)
    (else
      (if (`self.ActorHasTag` OtherActor "PistolTarget")
        (bind _asbp_target_actor (cast `/Game/Weapons/Pistol/BP_TargetActor` OtherActor)
          (:`then`
            (`/Game/Weapons/Pistol/BP_TargetActor.ShowHitFeedback` _asbp_target_actor))
          (:`CastFailed`
            _))
        (`|SpawnActorFromClass` "/Game/Weapons/Pistol/BP_PistolImpactBits.BP_PistolImpactBits_C" (`KismetMathLibrary.MakeTransform` _impactpoint (`KismetMathLibrary.MakeRotFromX` _impactnormal) (`KismetMathLibrary.MakeVector` 1.0 1.0 1.0)) "AlwaysSpawn" "MultiplyWithRoot" null null)
        (`PlayerController.ClientStartCameraShake` :`self` (`GameplayStatics.GetPlayerController` 0) :`Shake` "/Game/Weapons/Pistol/CS_PistolHit.CS_PistolHit_C" :`Scale` (`self.HitShakeScale`) :!label _label)
        (`GameplayStatics.PlaySoundAtLocation` (`self.HitSound`) _returnvalue (struct) 1.0 1.0 0.0 null null null null)
        (`GameplayStatics.SpawnEmitterAtLocation` (`self.ImpactEffect`) _returnvalue (struct) (`KismetMathLibrary.MakeVector` 1.0 1.0 1.0))
        (`KismetSystemLibrary.PrintString` "Pistol Target Hit" false))
      (`self.K2_DestroyActor`))))

(event `self.ReceiveActorBeginOverlap`
  (params (OtherActor :type "Actor Object Reference"))
  (bind _asbp_enemy_straight_runner (cast `/Game/Enemies/BP_EnemyStraightRunner` OtherActor))
  (`self.HandleEnemyOverlap`)
  (if (== (`self.WeaponKind`) 3)
    (`self.Detonate`)
    (else
      (`/Game/Enemies/BP_EnemyStraightRunner.Die` _asbp_enemy_straight_runner)
      (`|SpawnActorFromClass` "/Game/Weapons/Pistol/BP_PistolImpactBits.BP_PistolImpactBits_C" (`self.GetTransform`) "AlwaysSpawn" "MultiplyWithRoot" null null)
      (goto _label))))

(fn `BeginExplosionFeedback`
  (bind _returnvalue (`GameplayStatics.GetPlayerCharacter` 0))
  (bind _returnvalue_2 (`self.K2_GetActorLocation`))
  (bind _returnvalue_3 (`GameplayStatics.GetPlayerCameraManager` 0))
  (bind _returnvalue_4 (/ (`self.ExplosionCoreRadius`) 50.0))
  (bind _returnvalue_5 (/ (`self.ExplosionFlareRadius`) 50.0))
  (bind _returnvalue_6 (/ (`KismetMathLibrary.FClamp` (`self.BlastRadius`) 100.0 1000.0) 50.0))
  (`SceneComponent.SetVisibility` (`self.Tracer`) false false)
  (`MeshComponent.SetVectorParameterValueOnMaterials` (`self.ExplosionSphere`) "TracerColor" (3.0 0.9 0.08))
  (`SceneComponent.SetWorldScale3D` (`self.ExplosionSphere`) (`KismetMathLibrary.MakeVector` _returnvalue_4 _returnvalue_4 _returnvalue_4))
  (`PrimitiveComponent.SetCastShadow` (`self.ExplosionSphere`) false)
  (bind _returnvalue_7 (`self.AddComponentByClass` "/Script/Engine.StaticMeshComponent" true (`KismetMathLibrary.MakeTransform` (0.0 0.0 0.0) (struct) (1.0 1.0 1.0))))
  (bind `_as스태틱_메시_컴포넌트` (cast `StaticMeshComponent` _returnvalue_7))
  (set `self.ExplosionRing` `_as스태틱_메시_컴포넌트`)
  (`PrimitiveComponent.SetCollisionEnabled` (`self.ExplosionRing`) "NoCollision")
  (`StaticMeshComponent.SetStaticMesh` (`self.ExplosionRing`) "/Engine/BasicShapes/Plane.Plane")
  (`PrimitiveComponent.SetMaterial` (`self.ExplosionRing`) 0 "/Game/Enemies/Materials/M_AttackTelegraph.M_AttackTelegraph")
  (`SceneComponent.SetAbsolute` (`self.ExplosionRing`) true true true)
  (`SceneComponent.K2_SetWorldLocation` (`self.ExplosionRing`) (`KismetMathLibrary.MakeVector` (.x (`self.K2_GetActorLocation`)) (.y (`self.K2_GetActorLocation`)) (+ (- (.z (`self.K2_GetActorLocation` _returnvalue)) (`CapsuleComponent.GetScaledCapsuleHalfHeight` (`self.GetComponentByClass` _returnvalue "/Script/Engine.CapsuleComponent"))) 3.0)) false true)
  (`SceneComponent.K2_SetWorldRotation` :`self` (`self.ExplosionRing`) :`bTeleport` true)
  (`SceneComponent.SetWorldScale3D` (`self.ExplosionRing`) (`KismetMathLibrary.MakeVector` _returnvalue_6 _returnvalue_6 1.0))
  (`PrimitiveComponent.SetCastShadow` (`self.ExplosionRing`) false)
  (`MeshComponent.SetVectorParameterValueOnMaterials` (`self.ExplosionRing`) "TracerColor" (1.0 0.36 0.045))
  (`MeshComponent.SetScalarParameterValueOnMaterials` (`self.ExplosionRing`) "ShapeMode" 2.0)
  (`MeshComponent.SetScalarParameterValueOnMaterials` (`self.ExplosionRing`) "EffectProgress" 0.0)
  (`MeshComponent.SetScalarParameterValueOnMaterials` (`self.ExplosionRing`) "Opacity" 0.95)
  (`SceneComponent.SetVisibility` (`self.ExplosionRing`) true false)
  (bind _returnvalue_8 (`self.AddComponentByClass` "/Script/Engine.StaticMeshComponent" true (`KismetMathLibrary.MakeTransform` (0.0 0.0 0.0) (struct) (1.0 1.0 1.0))))
  (bind `_as스태틱_메시_컴포넌트_2` (cast `StaticMeshComponent` _returnvalue_8))
  (set `self.ExplosionFlare` `_as스태틱_메시_컴포넌트_2`)
  (`PrimitiveComponent.SetCollisionEnabled` (`self.ExplosionFlare`) "NoCollision")
  (`StaticMeshComponent.SetStaticMesh` (`self.ExplosionFlare`) "/Engine/BasicShapes/Plane.Plane")
  (`PrimitiveComponent.SetMaterial` (`self.ExplosionFlare`) 0 "/Game/Enemies/Materials/M_AttackTelegraph.M_AttackTelegraph")
  (`SceneComponent.SetAbsolute` (`self.ExplosionFlare`) true true true)
  (`SceneComponent.K2_SetWorldLocation` (`self.ExplosionFlare`) _returnvalue_2 false true)
  (`SceneComponent.K2_SetWorldRotation` (`self.ExplosionFlare`) (`KismetMathLibrary.MakeRotFromZX` (- (`PlayerCameraManager.GetCameraLocation` _returnvalue_3) _returnvalue_2) (`KismetMathLibrary.GetRightVector` (`PlayerCameraManager.GetCameraRotation` _returnvalue_3))) false true)
  (`SceneComponent.SetWorldScale3D` (`self.ExplosionFlare`) (`KismetMathLibrary.MakeVector` _returnvalue_5 _returnvalue_5 1.0))
  (`PrimitiveComponent.SetCastShadow` (`self.ExplosionFlare`) false)
  (`MeshComponent.SetVectorParameterValueOnMaterials` (`self.ExplosionFlare`) "TracerColor" (1.0 0.3 0.03))
  (`MeshComponent.SetScalarParameterValueOnMaterials` (`self.ExplosionFlare`) "ShapeMode" 3.0)
  (`MeshComponent.SetScalarParameterValueOnMaterials` (`self.ExplosionFlare`) "EffectProgress" 0.0)
  (`MeshComponent.SetScalarParameterValueOnMaterials` (`self.ExplosionFlare`) "Opacity" 0.95)
  (`SceneComponent.SetVisibility` (`self.ExplosionFlare`) true false))

(fn `ConfigureProjectile`
  (bind _projectilemovement (`self.ProjectileMovement`))
  (bind _projectilespeed (`self.ProjectileSpeed`))
  (bind _projectilemovement_2 (`self.ProjectileMovement`))
  (bind _projectilespeed_2 (`self.ProjectileSpeed`))
  (bind _projectilemovement_3 (`self.ProjectileMovement`))
  (bind _projectilespeed_3 (`self.ProjectileSpeed`))
  (bind _projectilemovement_4 (`self.ProjectileMovement`))
  (bind _projectilespeed_4 (`self.ProjectileSpeed`))
  (bind _returnvalue (/ (`KismetMathLibrary.FClamp` (`self.RocketRange`) 100.0 12000.0) _projectilespeed_4))
  (`PrimitiveComponent.IgnoreActorWhenMoving` (`self.Collision`) (`GameplayStatics.GetPlayerPawn` 0) true)
  (if (== (`self.WeaponKind`) 0)
    (set `self.ProjectileSpeed` 2200.0)
    (set `ProjectileMovementComponent.MaxSpeed` _projectilespeed _projectilemovement)
    (`ProjectileMovementComponent.SetVelocityInLocalSpace` _projectilemovement (`KismetMathLibrary.MakeVector` _projectilespeed))
    (`self.SetLifeSpan` (/ (`KismetMathLibrary.FClamp` (`self.PistolRange`) 100.0 12000.0) _projectilespeed))
    (elif (== (`self.WeaponKind`) 1)
      (set `self.ProjectileSpeed` 2200.0)
      (set `ProjectileMovementComponent.MaxSpeed` _projectilespeed_2 _projectilemovement_2)
      (`ProjectileMovementComponent.SetVelocityInLocalSpace` _projectilemovement_2 (`KismetMathLibrary.MakeVector` _projectilespeed_2))
      (`self.SetLifeSpan` (/ (`KismetMathLibrary.FClamp` (`self.ShotgunRange`) 100.0 12000.0) _projectilespeed_2))
      (elif (== (`self.WeaponKind`) 2)
        (set `self.ProjectileSpeed` 14000.0)
        (set `ProjectileMovementComponent.MaxSpeed` _projectilespeed_3 _projectilemovement_3)
        (`ProjectileMovementComponent.SetVelocityInLocalSpace` _projectilemovement_3 (`KismetMathLibrary.MakeVector` _projectilespeed_3))
        (`self.SetActorEnableCollision` false)
        (`self.SetLifeSpan` (/ (`KismetMathLibrary.FClamp` (`self.SniperRange`) 100.0 12000.0) _projectilespeed_3))
        (elif (== (`self.WeaponKind`) 3)
          (set `self.ProjectileSpeed` (`KismetMathLibrary.FClamp` (`self.RocketSpeed`) 400.0 4000.0))
          (set `ProjectileMovementComponent.MaxSpeed` _projectilespeed_4 _projectilemovement_4)
          (`ProjectileMovementComponent.SetVelocityInLocalSpace` _projectilemovement_4 (`KismetMathLibrary.MakeVector` _projectilespeed_4))
          (`KismetSystemLibrary.K2_SetTimer` self "Detonate" _returnvalue false true)
          (`self.SetLifeSpan` (- _returnvalue -0.4)))))))

(fn `Detonate`
  (bind _returnvalue (`self.K2_GetActorLocation`))
  (bind _returnvalue_2 (`KismetMathLibrary.MakeTransform` _returnvalue (struct) (3.0 3.0 3.0)))
  (if (not (`self.ExplosionDone`))
    (set `self.ExplosionDone` true)
    (`self.SetActorEnableCollision` false)
    (`MovementComponent.StopMovementImmediately` (`self.ProjectileMovement`))
    (`GameplayStatics.ApplyRadialDamage` 100.0 _returnvalue (`KismetMathLibrary.FClamp` (`self.BlastRadius`) 100.0 1000.0) null (`|MakeArray` (`self.GetOwner`) self (`self.GetInstigator`) (`GameplayStatics.GetPlayerPawn` 0) :!type "Actor Object Reference") self (`self.GetInstigatorController`) true "ECC_Camera")
    (bind _returnvalue_3 (`GameplayStatics.BeginDeferredActorSpawnFromClass` "/Game/Weapons/Pistol/BP_PistolImpactBits.BP_PistolImpactBits_C" _returnvalue_2 "AlwaysSpawn" null))
    (`GameplayStatics.FinishSpawningActor` _returnvalue_3 _returnvalue_2)
    (set `self.ExplosionStartTime` (`KismetSystemLibrary.GetGameTimeInSeconds`))
    (bind _returnvalue_4 (`self.AddComponentByClass` "/Script/Engine.StaticMeshComponent" false (`KismetMathLibrary.MakeTransform` (0.0 0.0 0.0))))
    (bind `_as스태틱_메시_컴포넌트` (cast `StaticMeshComponent` _returnvalue_4))
    (set `self.ExplosionSphere` `_as스태틱_메시_컴포넌트`)
    (`PrimitiveComponent.SetCollisionEnabled` `_as스태틱_메시_컴포넌트` "NoCollision")
    (`StaticMeshComponent.SetStaticMesh` `_as스태틱_메시_컴포넌트` "/Engine/BasicShapes/Sphere.Sphere")
    (`SceneComponent.SetRelativeScale3D` `_as스태틱_메시_컴포넌트` (0.1 0.1 0.1))
    (`SceneComponent.K2_SetRelativeRotation` :`self` `_as스태틱_메시_컴포넌트` :`bTeleport` true)
    (`SceneComponent.K2_SetRelativeLocation` `_as스태틱_메시_컴포넌트` (0.0 0.0 0.0) false true)
    (`PrimitiveComponent.SetMaterial` `_as스태틱_메시_컴포넌트` 0 "/Game/Weapons/Pistol/M_BulletTracer.M_BulletTracer")
    (`self.BeginExplosionFeedback`)
    (`KismetSystemLibrary.K2_SetTimer` self "UpdateExplosionVisual" 0.02 true true)
    (`self.SetLifeSpan` (+ (`KismetMathLibrary.FClamp` (`self.ExplosionVisualDuration`) 0.08) 0.07))))

(fn `HandleEnemyOverlap`)

(fn `HandleWeaponHit`)

(fn `UpdateExplosionVisual`
  (bind _returnvalue (`KismetMathLibrary.FClamp` (`self.ExplosionVisualDuration`) 0.08))
  (bind _returnvalue_2 (`KismetMathLibrary.FClamp` (`self.ExplosionCoreDuration`) 0.01 0.15))
  (bind _returnvalue_3 (- (`KismetSystemLibrary.GetGameTimeInSeconds`) (`self.ExplosionStartTime`)))
  (bind _returnvalue_4 (`KismetMathLibrary.FClamp` (/ _returnvalue_3 _returnvalue)))
  (bind _returnvalue_5 (* (/ (`self.ExplosionCoreRadius`) 50.0) (- 1.0 (* (`KismetMathLibrary.FClamp` (/ _returnvalue_3 _returnvalue_2)) 0.3))))
  (`MeshComponent.SetScalarParameterValueOnMaterials` (`self.ExplosionRing`) "EffectProgress" _returnvalue_4)
  (`MeshComponent.SetScalarParameterValueOnMaterials` (`self.ExplosionFlare`) "EffectProgress" _returnvalue_4)
  (if (>= _returnvalue_3 _returnvalue_2)
    (`SceneComponent.SetVisibility` (`self.ExplosionSphere`) false false)
    (else
      (`SceneComponent.SetWorldScale3D` (`self.ExplosionSphere`) (`KismetMathLibrary.MakeVector` _returnvalue_5 _returnvalue_5 _returnvalue_5))))
  (if (>= _returnvalue_3 _returnvalue)
    (`SceneComponent.SetVisibility` (`self.ExplosionRing`) false false)
    (`SceneComponent.SetVisibility` (`self.ExplosionSphere`) false false)
    (`SceneComponent.SetVisibility` (`self.ExplosionFlare`) false false)
    (`KismetSystemLibrary.K2_ClearTimer` self "UpdateExplosionVisual")))

(fn `UserConstructionScript`)
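; Pistol impact debris actor that scatters eight physics bits when spawned.
; On BeginPlay each bit gets a linear velocity along the actor's forward vector at BurstSpeed, plus a random unit direction scaled by SpreadSpeed.
; Each bit also gets its own fixed angular velocity so the pieces tumble differently.
; All motion is left to physics after that, with no tick or overlap logic.
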(event `self.ReceiveBeginPlay`
  (bind _burstspeed (`self.BurstSpeed`))
  (bind _spreadspeed (`self.SpreadSpeed`))
  (bind _bit0 (`self.Bit0`))
  (bind _bit1 (`self.Bit1`))
  (bind _bit2 (`self.Bit2`))
  (bind _bit3 (`self.Bit3`))
  (bind _bit4 (`self.Bit4`))
  (bind _bit5 (`self.Bit5`))
  (bind _bit6 (`self.Bit6`))
  (bind _bit7 (`self.Bit7`))
  (bind _returnvalue (`KismetMathLibrary.MakeVector` _burstspeed _burstspeed _burstspeed))
  (bind _returnvalue_2 (`KismetMathLibrary.MakeVector` _spreadspeed _spreadspeed _spreadspeed))
  (`PrimitiveComponent.SetPhysicsLinearVelocity` _bit0 (+ (* (`self.GetActorForwardVector`) _returnvalue) (* (`KismetMathLibrary.RandomUnitVector`) _returnvalue_2)) false "None")
  (`PrimitiveComponent.SetPhysicsAngularVelocityInDegrees` _bit0 (`KismetMathLibrary.MakeVector` 150.0 360.0 100.0) false "None")
  (`PrimitiveComponent.SetPhysicsLinearVelocity` _bit1 (+ (* (`self.GetActorForwardVector`) _returnvalue) (* (`KismetMathLibrary.RandomUnitVector`) _returnvalue_2)) false "None")
  (`PrimitiveComponent.SetPhysicsAngularVelocityInDegrees` _bit1 (`KismetMathLibrary.MakeVector` 230.0 325.0 145.0) false "None")
  (`PrimitiveComponent.SetPhysicsLinearVelocity` _bit2 (+ (* (`self.GetActorForwardVector`) _returnvalue) (* (`KismetMathLibrary.RandomUnitVector`) _returnvalue_2)) false "None")
  (`PrimitiveComponent.SetPhysicsAngularVelocityInDegrees` _bit2 (`KismetMathLibrary.MakeVector` 310.0 290.0 190.0) false "None")
  (`PrimitiveComponent.SetPhysicsLinearVelocity` _bit3 (+ (* (`self.GetActorForwardVector`) _returnvalue) (* (`KismetMathLibrary.RandomUnitVector`) _returnvalue_2)) false "None")
  (`PrimitiveComponent.SetPhysicsAngularVelocityInDegrees` _bit3 (`KismetMathLibrary.MakeVector` 390.0 255.0 235.0) false "None")
  (`PrimitiveComponent.SetPhysicsLinearVelocity` _bit4 (+ (* (`self.GetActorForwardVector`) _returnvalue) (* (`KismetMathLibrary.RandomUnitVector`) _returnvalue_2)) false "None")
  (`PrimitiveComponent.SetPhysicsAngularVelocityInDegrees` _bit4 (`KismetMathLibrary.MakeVector` 470.0 220.0 280.0) false "None")
  (`PrimitiveComponent.SetPhysicsLinearVelocity` _bit5 (+ (* (`self.GetActorForwardVector`) _returnvalue) (* (`KismetMathLibrary.RandomUnitVector`) _returnvalue_2)) false "None")
  (`PrimitiveComponent.SetPhysicsAngularVelocityInDegrees` _bit5 (`KismetMathLibrary.MakeVector` 550.0 185.0 325.0) false "None")
  (`PrimitiveComponent.SetPhysicsLinearVelocity` _bit6 (+ (* (`self.GetActorForwardVector`) _returnvalue) (* (`KismetMathLibrary.RandomUnitVector`) _returnvalue_2)) false "None")
  (`PrimitiveComponent.SetPhysicsAngularVelocityInDegrees` _bit6 (`KismetMathLibrary.MakeVector` 630.0 150.0 370.0) false "None")
  (`PrimitiveComponent.SetPhysicsLinearVelocity` _bit7 (+ (* (`self.GetActorForwardVector`) _returnvalue) (* (`KismetMathLibrary.RandomUnitVector`) _returnvalue_2)) false "None")
  (`PrimitiveComponent.SetPhysicsAngularVelocityInDegrees` _bit7 (`KismetMathLibrary.MakeVector` 710.0 115.0 415.0) false "None"))

(fn `UserConstructionScript`)
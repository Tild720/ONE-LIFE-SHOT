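; BP_RunnerProgress is an actor that tracks how far the player has run between StartPoint and EndPoint and owns the progress HUD widget.
; A looping timer, used instead of Tick, projects the player pawn onto the straight start-to-end line to get clamped Progress and RemainingDistance.
; Progress thresholds select one of five E_RunnerStage values, and OnStageChanged fires when the stage changes.
; WBP_RunnerProgress is added on BeginPlay and removed on EndPlay.
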(event `self.ReceiveBeginPlay`
  (`self.UpdateProgress`)
  (`KismetSystemLibrary.K2_SetTimer` self "UpdateProgress" (`KismetMathLibrary.FClamp` (`self.UpdateInterval`) 0.05) true)
  (bind _returnvalue (`|CreateWidget` "/Game/UI/WBP_RunnerProgress.WBP_RunnerProgress_C" (`GameplayStatics.GetPlayerController` 0)))
  (set `self.ProgressHUD` _returnvalue)
  (`UserWidget.AddToViewport` _returnvalue 10))

(event `self.ReceiveEndPlay`
  (params (EndPlayReason :type "EEndPlayReason Enum" :default "Destroyed"))
  (`KismetSystemLibrary.K2_ClearTimer` self "UpdateProgress")
  (`/Engine/EditorBlueprintResources/StandardMacros.IsValid` (`self.ProgressHUD`)
    (:`Is Valid`
      (`Widget.RemoveFromParent` (`self.ProgressHUD`)))))

(fn `UpdateProgress`
  (bind _returnvalue (`GameplayStatics.GetPlayerPawn` 0))
  (`/Engine/EditorBlueprintResources/StandardMacros.IsValid` _returnvalue
    (:`Is Valid`
      (`/Engine/EditorBlueprintResources/StandardMacros.IsValid` (`self.StartPoint`)
        (:`Is Valid`
          (`/Engine/EditorBlueprintResources/StandardMacros.IsValid` (`self.EndPoint`)
            (:`Is Valid`
              (set `self.TrackLength` (`KismetMathLibrary.VSize` (- (`self.K2_GetActorLocation` (`self.EndPoint`)) (`self.K2_GetActorLocation` (`self.StartPoint`)))))
              (if (> (`self.TrackLength`) 1.0)
                (set `self.Progress` (`KismetMathLibrary.FClamp` (/ (`KismetMathLibrary.Dot_VectorVector` (- (`self.K2_GetActorLocation` _returnvalue) (`self.K2_GetActorLocation` (`self.StartPoint`))) (- (`self.K2_GetActorLocation` (`self.EndPoint`)) (`self.K2_GetActorLocation` (`self.StartPoint`)))) (* (`self.TrackLength`) (`self.TrackLength`)))))
                (set `self.RemainingDistance` (* (- 1.0 (`self.Progress`)) (`self.TrackLength`)))
                (set `self.PreviousStage` (`self.CurrentStage`))
                (set `self.CurrentStage` (select `bool` (>= (`self.Progress`) 1.0) :`false` (select `bool` (>= (`self.Progress`) (`self.FinalThreshold`)) :`false` (select `bool` (>= (`self.Progress`) (`self.LateThreshold`)) :`false` (select `bool` (>= (`self.Progress`) (`self.MiddleThreshold`)) :`false` (enumliteral `/Game/Runner/E_RunnerStage` "NewEnumerator0") :`true` (enumliteral `/Game/Runner/E_RunnerStage` "NewEnumerator1")) :`true` (enumliteral `/Game/Runner/E_RunnerStage` "NewEnumerator2")) :`true` (enumliteral `/Game/Runner/E_RunnerStage` "NewEnumerator3")) :`true` (enumliteral `/Game/Runner/E_RunnerStage` "NewEnumerator4")))
                (if (not (`|EnumEquality` (`self.PreviousStage`) (`self.CurrentStage`)))
                  (`self.OnStageChanged`))))))))))

(fn `UserConstructionScript`)